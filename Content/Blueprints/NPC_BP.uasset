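; NPC Blueprint that chases the player's active projectile and destroys it on reaching it.
; Each tick it reads the projectile flag and reference from Player_BP, smoothly rotates toward the projectile and applies forward movement input.
; Within a short distance it destroys the projectile and clears the player's IsProjectileOut flag.
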(event EventTick
  (params (DeltaSeconds :type Float%20%28single-precision%29))
  (bind _returnvalue (Transformation|GetActorRotation))
  (bind _mesh (Variables|Character|GetMesh))
  (bind _returnvalue_2 (Transformation|GetWorldLocation _mesh))
  (bind _asplayer_bp (Utilities|Casting|CastToPlayer_BP (Game|Player|GetPlayerPawn 0)))
  (if (Variables|/Game/Blueprints/Player_BP.Player_BP_C|GetIsProjectileOut _asplayer_bp)
    (if (> (Math|Vector|Distance(Vector) _returnvalue_2 (Transformation|GetWorldLocation (Variables|/Game/Blueprints/Projectile_BP.Projectile_BP_C|GetSphere (Variables|/Game/Blueprints/Player_BP.Player_BP_C|GetProjectile _asplayer_bp)))) 1e+02)
      (Transformation|SetActorRotation (Math|Interpolation|RInterpTo _returnvalue (Math|Rotator|FindLookatRotation _returnvalue_2 (Transformation|GetWorldLocation (Variables|/Game/Blueprints/Projectile_BP.Projectile_BP_C|GetSphere (Variables|/Game/Blueprints/Player_BP.Player_BP_C|GetProjectile _asplayer_bp)))) (Utilities|Time|GetWorldDeltaSeconds) 5.0))
      (Variables|Default|SetscaleValue 1.0)
      (Pawn|Input|AddMovementInput (Math|Vector|GetForwardVector _returnvalue) (Variables|Default|GetscaleValue) false)
      (else
        (Actor|DestroyActor (Variables|/Game/Blueprints/Player_BP.Player_BP_C|GetProjectile _asplayer_bp))
        (bind _asplayer_bp_2 (Utilities|Casting|CastToPlayer_BP (Game|Player|GetPlayerPawn 0)))
        (Variables|/Game/Blueprints/Player_BP.Player_BP_C|SetIsProjectileOut _asplayer_bp_2 false)))))

(fn ConstructionScript)